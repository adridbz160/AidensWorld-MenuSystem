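; Player controller that handles pausing and the collect menu for the Aiden character.
; On BeginPlay it caches the player character and the in-game HUD, which shows and removes both menus.
; The pause input toggles game pause, while the collect input uses a FlipFlop to open or close its menu, disabling the character's camera movement while open.
; Both inputs are ignored while the character's loading screen is valid.
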(event Input|EnhancedActionEvents|EnhancedInputActionIA_Pause
  (params (ActionValue :type Boolean) (ElapsedSeconds :type Float%20%28double-precision%29) (TriggeredSeconds :type Float%20%28double-precision%29) (InputAction :type Input%20Action%20Object%20Reference :default "/Game/Blueprints/Character/Input/Actions/IA_Pause.IA_Pause"))
  (bind _self self)
  (:Started
    (Variables|/Game/Blueprints/Character/Blueprints/BP_AidenCharacter.BP_AidenCharacter_C|GetloadingScreen? (Variables|Default|GetAs%20BP%20Aiden%20Character)
      (:then)
      (:else
        (if (Game|IsGamePaused)
          (CallFunction|ResumeGame _self)
          (else
            (CallFunction|PauseGame _self)))))))

(event Input|EnhancedActionEvents|EnhancedInputActionIA_Collect
  (params (ActionValue :type Boolean) (ElapsedSeconds :type Float%20%28double-precision%29) (TriggeredSeconds :type Float%20%28double-precision%29) (InputAction :type Input%20Action%20Object%20Reference :default "/Game/Blueprints/Character/Input/Actions/IA_Collect.IA_Collect"))
  (bind _self self)
  (:Started
    (Variables|/Game/Blueprints/Character/Blueprints/BP_AidenCharacter.BP_AidenCharacter_C|GetloadingScreen? (Variables|Default|GetAs%20BP%20Aiden%20Character)
      (:then)
      (:else
        (Utilities|FlowControl|FlipFlop
          (:A
            (Default|CollectMenuShow _self))
          (:B
            (Default|CollectMenuClose _self)))))))

(event EventCollectMenuShow
  (bind _hudingame (Variables|Default|GetHUDInGame)
    (:then
      (Variables|/Game/Blueprints/Character/Blueprints/BP_AidenCharacter.BP_AidenCharacter_C|SetcameraMovement? (Variables|Default|GetAs%20BP%20Aiden%20Character) false)
      (Variables|Default|SetOpen? true)
      (Default|ShowCollectMenu _hudingame))
    (:else)))

(event EventCollectMenuClose
  (bind _hudingame (Variables|Default|GetHUDInGame)
    (:then
      (Variables|/Game/Blueprints/Character/Blueprints/BP_AidenCharacter.BP_AidenCharacter_C|SetcameraMovement? (Variables|Default|GetAs%20BP%20Aiden%20Character) true)
      (Variables|Default|SetOpen? false)
      (Default|RemoveCollectMenu _hudingame))
    (:else)))

(event EventBeginPlay
  (bind _asbp_aiden_character (Utilities|Casting|CastToBP_AidenCharacter (Game|GetPlayerCharacter 0)))
  (Variables|Default|SetAs%20BP%20Aiden%20Character _asbp_aiden_character)
  (bind _ashud_in_game (Utilities|Casting|CastToHUD_InGame (HUD|GetHUD)))
  (Variables|Default|SetHUDInGame _ashud_in_game))

(event EventPauseGame
  (Game|SetGamePaused true)
  (bind _hudingame (Variables|Default|GetHUDInGame)
    (:then
      (Default|ShowPauseMenu _hudingame))
    (:else)))

(event EventResumeGame
  (Game|SetGamePaused false)
  (bind _hudingame (Variables|Default|GetHUDInGame)
    (:then
      (Default|RemovePauseMenu _hudingame))
    (:else)))

(fn ConstructionScript)