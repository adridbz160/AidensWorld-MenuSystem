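; BP_SpawnBlock is a pressure plate companion block that grows or shrinks vertically by scaling its SMPressurePlatePrompt component.
; BeginPlay converts LocationOffset into a Z-scale range, with IsReversed starting the block extended so it collapses instead of growing.
; TriggerAnimation clears IsActivated and flips RegularExecution to alternate between playing and reversing the Move timeline, which lerps the Z scale between both ends.
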(event Custom|TriggerAnimation
  ;[1 1 1] Trigger animation
  (Variables|Default|SetisActivated? false)
  (bind _output_get (Variables|Default|SetregularExecution? (Variables|Default|GetregularExecution?)))
  (if _output_get
    (Variables|Default|SetregularExecution? (not _output_get))
    (CallFunction|Play)
    (else
      (Variables|Default|SetregularExecution? (not _output_get))
      (CallFunction|Reverse))))

(event Custom|Reverse
  (bind _sm_pressureplateprompt (Variables|Default|GetSM_PressurePlatePrompt))
  (bind _returnvalue (Transformation|GetWorldScale _sm_pressureplateprompt))
  ;[1 1 1] Scaling animation
  (bind _alpha (Timeline|Move Reverse)
    (:Update
      (Transformation|SetWorldScale3D _sm_pressureplateprompt (Math|Vector|MakeVector (.x _returnvalue) (.y _returnvalue) (Math|Float|Lerp (Variables|Default|GetinitialLocationZ) (Variables|Default|GetlocationOffset) _alpha))))))

(event Custom|Play
  (bind _sm_pressureplateprompt (Variables|Default|GetSM_PressurePlatePrompt))
  (bind _returnvalue (Transformation|GetWorldScale _sm_pressureplateprompt))
  ;[1 1 1] Scaling animation
  (bind _alpha (Timeline|Move Play)
    (:Update
      (Transformation|SetWorldScale3D _sm_pressureplateprompt (Math|Vector|MakeVector (.x _returnvalue) (.y _returnvalue) (Math|Float|Lerp (Variables|Default|GetinitialLocationZ) (Variables|Default|GetlocationOffset) _alpha))))))

(event EventBeginPlay
  (bind _sm_pressureplateprompt (Variables|Default|GetSM_PressurePlatePrompt))
  (bind _returnvalue (Transformation|GetWorldScale _sm_pressureplateprompt))
  ;[1 1 1] Initialize scale
  (if (Variables|Default|GetisReversed?)
    (Transformation|SetWorldScale3D _sm_pressureplateprompt (Math|Vector|MakeVector (.x _returnvalue) (.y _returnvalue) (* (Variables|Default|GetlocationOffset) 0.005)))
    (Variables|Default|SetinitialLocationZ (* (Variables|Default|GetlocationOffset) 0.005))
    (Variables|Default|SetlocationOffset 0.0)
    (else
      (Variables|Default|SetinitialLocationZ 0.0)
      (Variables|Default|SetlocationOffset (* (Variables|Default|GetlocationOffset) 0.005)))))

(fn ConstructionScript)