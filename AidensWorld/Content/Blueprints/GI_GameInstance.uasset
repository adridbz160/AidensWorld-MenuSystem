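; Game instance that owns the user's settings save game and persists audio settings to a save slot.
; LoadSettings returns the cached SG_UserSettings object, first loading it from the slot or creating a new one if no save exists.
; SaveAudioSettings writes the audio settings into that object, then calls SaveSettings, which saves it to the slot and prints whether it succeeded.
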(fn SaveAudioSettings
  (params (AudioSettings :type S%20Audio%20Settings%20Structure))
  (Variables|/Game/UI/Blueprints/SaveGame/SG_UserSettings.SG_UserSettings_C|SetAudioSettings (CallFunction|LoadSettings) AudioSettings)
  (CallFunction|SaveSettings))

(fn LoadSettings
  (bind _settingssaveslot (Variables|Default|GetSettingsSaveSlot))
  (Variables|Default|GetSGUserSettings
    (:then
      _)
    (:else
      (bind _returnvalue (SaveGame|DoesSaveGameExist _settingssaveslot))
      (if _returnvalue
        (bind _returnvalue_2 (SaveGame|LoadGamefromSlot _settingssaveslot))
        (bind _assg_user_settings (Utilities|Casting|CastToSG_UserSettings _returnvalue_2))
        (Variables|Default|SetSGUserSettings _assg_user_settings)
        (else
          (bind _returnvalue_3 (SaveGame|CreateSaveGameObject (Variables|Default|GetSGUserSettingsClass)))
          (bind _assg_user_settings_2 (Utilities|Casting|CastToSG_UserSettings _returnvalue_3))
          (Variables|Default|SetSGUserSettings _assg_user_settings_2)))))
  (return (Variables|Default|GetSGUserSettings)))

(fn SaveSettings
  (bind _returnvalue (SaveGame|SaveGametoSlot (Variables|Default|GetSGUserSettings) (Variables|Default|GetSettingsSaveSlot)))
  (Development|PrintString (Utilities|String|Append "Settings Saved: " (Utilities|String|ToString(Boolean) _returnvalue)) true true "(R=0.000000,G=0.660000,B=1.000000,A=1.000000)" 5.0))